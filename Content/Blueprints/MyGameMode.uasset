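; Game mode that sets the sound mix at level start and runs the mission end sequence.
; BeginPlay clears sound mix modifiers and pushes a mute SFX mix.
; Mission completion and failure share one sequence that signals game end, disables player input, hides the objective marker, fades out camera and SFX, then opens Level_01_ALL after timed delays.
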(event Custom|OnMissionCompleted
  (Default|CallOnGameEnd)
  (Input|DisableInput (CallFunction|GetMyPlayerCharacter) (Game|GetPlayerController 0))
  (Utilities|FlowControl|Delay 2.0)
  (Default|DeactivateObjectiveMarker (CallFunction|GetMissionManager))
  (CameraFades|StartCameraFade :self (Game|GetPlayerCameraManager 0) :ToAlpha 1.0 :Duration 2.0 :bHoldWhenFinished true)
  (Audio|PushSoundMixModifier "/Game/Audio/Sounds/Mixes/FadeOutSFX_SoundMix.FadeOutSFX_SoundMix")
  (Utilities|FlowControl|Delay 3.0)
  (Game|OpenLevel(byName) "Level_01_ALL"))

(event Custom|OnMissionFailed
  (Default|CallOnGameEnd)
  (Input|DisableInput (CallFunction|GetMyPlayerCharacter) (Game|GetPlayerController 0))
  (Utilities|FlowControl|Delay 2.0)
  (Default|DeactivateObjectiveMarker (CallFunction|GetMissionManager))
  (CameraFades|StartCameraFade :self (Game|GetPlayerCameraManager 0) :ToAlpha 1.0 :Duration 2.0 :bHoldWhenFinished true)
  (Audio|PushSoundMixModifier "/Game/Audio/Sounds/Mixes/FadeOutSFX_SoundMix.FadeOutSFX_SoundMix")
  (Utilities|FlowControl|Delay 3.0)
  (Game|OpenLevel(byName) "Level_01_ALL"))

(event EventBeginPlay
  (Class|GameplayStatics|ClearSoundMixModifiers)
  (Audio|PushSoundMixModifier "/Game/Audio/Sounds/Mixes/MuteSFX_SoundMix.MuteSFX_SoundMix"))

(fn ConstructionScript)