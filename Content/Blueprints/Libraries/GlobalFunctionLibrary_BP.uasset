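; GlobalFunctionLibrary_BP is a Blueprint function library of shortcuts to the game's core objects.
; GetMyGameMode casts the current game mode to MyGameMode_BP, and GetMissionManager reads the MissionManager from that result.
; GetMyPlayerCharacter casts the pawn of the first player to MyPlayerCharacter_BP.
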(fn GetMyGameMode
  (bind _asmy_game_mode_bp (Utilities|Casting|CastToMyGameMode_BP (Game|GetGameMode)))
  (return _asmy_game_mode_bp))

(fn GetMissionManager
  (return (Variables|/Game/Blueprints/MyGameMode_BP.MyGameMode_BP_C|GetMissionManager (CallFunction|GetMyGameMode))))

(fn GetMyPlayerCharacter
  (bind _asmy_player_character_bp (Utilities|Casting|CastToMyPlayerCharacter_BP (Game|Player|GetPlayerPawn 0)))
  (return _asmy_player_character_bp))