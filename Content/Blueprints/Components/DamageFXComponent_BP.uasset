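; An actor component that switches on damage particle effects in stages as its owner's health drops.
; On BeginPlay it caches the owner's HealthComponent and binds to OnTakeAnyDamage, or prints a warning if none exists.
; Particles are supplied through InitDamageFX; each damage event activates at most one, when health percentage falls below the current threshold.
; The threshold index then advances, and the damage event is unbound once it reaches the particle count.
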(event Custom|OnTakeAnyDamage_Event_0
  (params (DamagedActor :type Actor%20Object%20Reference) (Damage :type Float%20%28single-precision%29) (DamageType :type Damage%20Type%20Object%20Reference) (InstigatedBy :type Controller%20Object%20Reference) (DamageCauser :type Actor%20Object%20Reference))
  ;[0 1 0.03488] Damage FX
  (if (> (Utilities|Array|Length (Variables|Default|GetDamage%20Particles)) 0)
    (if (< (Class|HealthComponent|GetHealthPercentage (Variables|Default|GetHealthComp)) (Utilities|Array|Get(acopy) (Variables|Default|GetDamageTresholds) (Variables|Default|GetCurrentDamageTreshold)))
      (Components|Activation|Activate (Utilities|Array|Get(acopy) (Variables|Default|GetDamage%20Particles) (Variables|Default|GetCurrentDamageTreshold)) false)
      (bind _result (Math|Integer|IncrementInt (Variables|Default|GetCurrentDamageTreshold))
        (:%20%20
          (if (== _result (Utilities|Array|Length (Variables|Default|GetDamage%20Particles)))
            (EventDispatchers|UnbindEventfromOnTakeAnyDamage (Components|GetOwner) (EventDispatchers|CreateEvent :!event Custom|OnTakeAnyDamage_Event_0))))))))

(event Custom|InitDamageFX
  (params (DamageParticles :type Array%20of%20Particle%20System%20Component%20Object%20References))
  (Variables|Default|SetDamage%20Particles DamageParticles))

(event EventBeginPlay
  (bind _returnvalue (Components|GetOwner))
  (bind _returnvalue_2 (Actor|GetComponentbyClass _returnvalue "/Script/Game_02.HealthComponent"))
  (Utilities|IsValid _returnvalue_2
    (:Is%20Valid
      (Variables|Default|SetHealthComp _returnvalue_2)
      (EventDispatchers|AssignOnTakeAnyDamage _returnvalue (EventDispatchers|CreateEvent :!event Custom|OnTakeAnyDamage_Event_0)))
    (:Is%20Not%20Valid
      (Development|PrintString (Utilities|String|Append (Utilities|GetDisplayName _returnvalue) " has no Health Component!")))))