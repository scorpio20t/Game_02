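; Mission manager component that runs the game's current mission and reports its progress to the player HUD.
; Activation spawns the mission class as an actor only when no valid current mission exists, then initializes it.
; Stage changes, completion and failure require matching class and state; completion and failure set the same end state and notify the game mode.
; It also swaps or clears the mission's single objective marker, disabling the old one.
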(fn ActivateMission
  (params (Mission :type Mission%20Actor%20BP%20Class%20Reference))
  (Utilities|IsValid (Variables|Default|GetCurrentMission)
    (:Is%20Not%20Valid
      (bind _returnvalue (Game|SpawnActorfromClass Mission (Math|Transform|MakeTransform "0, 0, 0") "Undefined" 0 0))
      (bind _output_get (Variables|Default|SetCurrentMission _returnvalue))
      (Default|InitMission _output_get)
      (Default|OnMissionActivated (Variables|Default|GetPlayerHUD) (Variables|Default|GetCurrentMission)))))

(fn ChangeMissionStage
  (params (Mission :type Mission%20Actor%20BP%20Class%20Reference) (NewStage :type Integer))
  (bind _currentmission (Variables|Default|GetCurrentMission))
  (Utilities|IsValid _currentmission
    (:Is%20Valid
      (if (and (== Mission (Utilities|GetClass _currentmission)) (Utilities|Enum|Equal(Enum) (Variables|/Game/Blueprints/Objectives/MissionActor_BP.MissionActor_BP_C|GetMissionState _currentmission) "NewEnumerator1"))
        (Variables|/Game/Blueprints/Objectives/MissionActor_BP.MissionActor_BP_C|SetCurrentStage _currentmission NewStage)
        (Default|OnMissionStageChanged (Variables|Default|GetPlayerHUD) (Variables|Default|GetCurrentMission))))))

(fn CompleteMission
  (params (Mission :type Mission%20Actor%20BP%20Class%20Reference))
  (bind _currentmission (Variables|Default|GetCurrentMission))
  (Utilities|IsValid _currentmission
    (:Is%20Valid
      (if (and (== Mission (Utilities|GetClass _currentmission)) (Utilities|Enum|Equal(Enum) (Variables|/Game/Blueprints/Objectives/MissionActor_BP.MissionActor_BP_C|GetMissionState _currentmission) "NewEnumerator1"))
        (Variables|/Game/Blueprints/Objectives/MissionActor_BP.MissionActor_BP_C|SetMissionState _currentmission "NewEnumerator2")
        (Default|OnMissionCompleted (Variables|Default|GetPlayerHUD) (Variables|Default|GetCurrentMission))
        (Default|OnMissionCompleted (CallFunction|GetMyGameMode))))))

(fn FailMission
  (params (Mission :type Blueprint%20Rush%20Mission%20BP%20Class%20Reference))
  (bind _currentmission (Variables|Default|GetCurrentMission))
  (Utilities|IsValid _currentmission
    (:Is%20Valid
      (if (and (== Mission (Utilities|GetClass _currentmission)) (Utilities|Enum|Equal(Enum) (Variables|/Game/Blueprints/Objectives/MissionActor_BP.MissionActor_BP_C|GetMissionState _currentmission) "NewEnumerator1"))
        (Variables|/Game/Blueprints/Objectives/MissionActor_BP.MissionActor_BP_C|SetMissionState _currentmission "NewEnumerator2")
        (Default|OnMissionFailed (Variables|Default|GetPlayerHUD) (Variables|Default|GetCurrentMission))
        (Default|OnMissionFailed (CallFunction|GetMyGameMode))))))

(fn ActivateObjectiveMarker
  (params (ObjectiveMarker :type Objective%20Marker%20BP%20Object%20Reference))
  (bind _currentmission (Variables|Default|GetCurrentMission))
  (Utilities|IsValid _currentmission
    (:Is%20Valid
      (Utilities|IsValid (Variables|/Game/Blueprints/Objectives/MissionActor_BP.MissionActor_BP_C|GetObjectiveMarker _currentmission)
        (:Is%20Valid
          (Default|Disable (Variables|/Game/Blueprints/Objectives/MissionActor_BP.MissionActor_BP_C|GetObjectiveMarker _currentmission)))
        (:Is%20Not%20Valid
          _))
      (bind _output_get (Variables|/Game/Blueprints/Objectives/MissionActor_BP.MissionActor_BP_C|SetObjectiveMarker _currentmission ObjectiveMarker))
      (Default|ActivateObjectiveMarker (Variables|Default|GetPlayerHUD) _output_get))))

(fn DeactivateObjectiveMarker
  (bind _currentmission (Variables|Default|GetCurrentMission))
  (Utilities|IsValid _currentmission
    (:Is%20Valid
      (Utilities|IsValid (Variables|/Game/Blueprints/Objectives/MissionActor_BP.MissionActor_BP_C|GetObjectiveMarker _currentmission)
        (:Is%20Valid
          (Default|Disable (Variables|/Game/Blueprints/Objectives/MissionActor_BP.MissionActor_BP_C|GetObjectiveMarker _currentmission))
          (Variables|/Game/Blueprints/Objectives/MissionActor_BP.MissionActor_BP_C|SetObjectiveMarker _currentmission 0)
          (Default|DeactivateObjectiveMarker (Variables|Default|GetPlayerHUD)))))))