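; AI controller for the Evil Capsuloid enemy, extending a base enemy controller with its own behavior tree choice and smooth turning.
; On possess it runs a background-waypoint or patrol behavior tree and passes on any valid start waypoint.
; Each tick it interpolates rotation toward the target with line of fire, the movement direction without it, or control rotation when untargeted.
; Assigning a target also turns the capsuloid's spotlight red.
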(event EventPossess
  (params (PossessedPawn :type Pawn%20Object%20Reference))
  ;[1 1 1] Base Class override
  (bind _asenemy_base_bp (Utilities|Casting|CastToEnemyBase_BP PossessedPawn))
  (bind _output_get (Variables|Default|SetEnemyBase _asenemy_base_bp))
  (bind _asevil_capsuloid_bp (Utilities|Casting|CastToEvilCapsuloid_BP _output_get))
  (Variables|Default|SetEvilCapsuleoid _asevil_capsuloid_bp)
  (if (Variables|/Game/Blueprints/Pawns/Enemies/EvilCapsuloid_BP.EvilCapsuloid_BP_C|GetbBackgroundWaypoints (Variables|Default|GetEvilCapsuleoid))
    (AI|RunBehaviorTree "/Game/Blueprints/AI/Enemies/EvilCapsuloidBackgroundWaypoints_BT.EvilCapsuloidBackgroundWaypoints_BT")
    (else
      (AI|RunBehaviorTree "/Game/Blueprints/AI/Enemies/EvilCapsuloidPatrol_BT.EvilCapsuloidPatrol_BT")))
  (Utilities|IsValid (Variables|/Game/Blueprints/Pawns/Enemies/EnemyBase_BP.EnemyBase_BP_C|GetStartWaypoint (Variables|Default|GetEnemyBase))
    (:Is%20Valid
      (CallFunction|SetStartWaypoint (Variables|/Game/Blueprints/Pawns/Enemies/EnemyBase_BP.EnemyBase_BP_C|GetStartWaypoint (Variables|Default|GetEnemyBase))))))

(event EventTick
  (params (DeltaSeconds :type Float%20%28single-precision%29))
  ;[1 1 1] Smooth rotation handling
  (Utilities|IsValid (Variables|Default|GetCurrentTarget)
    (:Is%20Valid
      (if (ScalableFloat|GetValueasBool (Variables|Default|GetBlackboard) (Variables|Default|GetHasLineOfFireKey))
        (Transformation|SetActorRotation (Variables|Default|GetEnemyBase) (CallFunction|GetInterpolationtoTargetLoc))
        (else
          (Transformation|SetActorRotation (Variables|Default|GetEnemyBase) (CallFunction|GetInterpolationtoMovementDir)))))
    (:Is%20Not%20Valid
      (Transformation|SetActorRotation (Variables|Default|GetEnemyBase) (CallFunction|GetInterpolationtoControlRot)))))

(fn ConstructionScript
  (|CallParentFunction))

(fn AssignTarget
  (params (ObjectValue :type Object%20Object%20Reference))
  (|CallParentFunction ObjectValue)
  (Default|ChangeSpotlightColor (Variables|Default|GetEvilCapsuleoid) "(R=1.000000,G=0.000000,B=0.000000,A=1.000000)"))

(fn GetInterpolationtoMovementDir
  (return (Math|Interpolation|RInterpTo (Transformation|GetActorRotation (Variables|Default|GetEnemyBase)) (Math|Rotator|MakeRotator 0.0 0.0 (.yaw (Math|Conversions|RotationFromXVector (Transformation|GetVelocity (Variables|Default|GetEnemyBase))))) (Utilities|Time|GetWorldDeltaSeconds) (Variables|/Script/Engine.FloatingPawnMovement|GetTurningBoost (Variables|/Game/Blueprints/Pawns/Enemies/EnemyBase_BP.EnemyBase_BP_C|GetFloatingPawnMovement (Variables|Default|GetEnemyBase))))))

(fn GetInterpolationtoControlRot
  (return (Math|Interpolation|RInterpTo (Transformation|GetActorRotation (Variables|Default|GetEnemyBase)) (Pawn|GetControlRotation :!class /Script/Engine.Controller) (Utilities|Time|GetWorldDeltaSeconds) (Variables|/Script/Engine.FloatingPawnMovement|GetTurningBoost (Variables|/Game/Blueprints/Pawns/Enemies/EnemyBase_BP.EnemyBase_BP_C|GetFloatingPawnMovement (Variables|Default|GetEnemyBase))))))

(fn GetInterpolationtoTargetLoc
  (return (Math|Interpolation|RInterpTo (Transformation|GetActorRotation (Variables|Default|GetEnemyBase)) (Math|Rotator|MakeRotator 0.0 0.0 (.yaw (Math|Rotator|FindLookatRotation (Transformation|GetActorLocation (Variables|Default|GetEnemyBase)) (Transformation|GetActorLocation (Variables|Default|GetCurrentTarget))))) (Utilities|Time|GetWorldDeltaSeconds) (Variables|/Script/Engine.FloatingPawnMovement|GetTurningBoost (Variables|/Game/Blueprints/Pawns/Enemies/EnemyBase_BP.EnemyBase_BP_C|GetFloatingPawnMovement (Variables|Default|GetEnemyBase))))))