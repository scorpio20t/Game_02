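; Base AI controller for enemy pawns that runs a behavior tree and tracks hostile targets through AI perception.
; On possess it seeds the blackboard with the enemy's start waypoint, and on pawn death it stops the brain and disables sight.
; Sensed actors of another team join a target list; the first becomes current.
; A looping timer, with its interval randomized once, then reassigns a random target from that list.
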(event OnTargetPerceptionUpdated(AIPerception)
  (params (Actor :type Actor%20Object%20Reference) (Stimulus :type AI%20Stimulus%20Structure))
  ;[1 1 1] Detecting hostiles
  (if (.bSuccessfullySensed (Utilities|Struct|BreakAIStimulus Stimulus))
    (bind _teamtype (Class|TeamInterfaceBP|GetTeamType(Message) Actor))
    (if (Utilities|Enum|NotEqual(Enum) _teamtype (Variables|/Game/Blueprints/Pawns/Enemies/EnemyBase_BP.EnemyBase_BP_C|GetTeamType (Variables|Default|GetEnemyBase)))
      (Utilities|FlowControl|Sequence
        (:then_0
          (if (== (Utilities|Array|Length (Variables|Default|GetTargets)) 0)
            (CallFunction|AssignTarget Actor)))
        (:then_1
          (CallFunction|AddNewTarget Actor))))))

(event Custom|OnPawnDeath
  (AI|Logic|StopLogic (Variables|Default|GetBrainComponent) "")
  (Class|AIPerceptionComponent|SetSenseEnabled (Variables|Default|GetAIPerception) "/Script/AIModule.AISense_Sight" false))

(event Custom|InitiateTargeting
  ;[1 1 1] Switching targets
  (if (not (Variables|Default|GetbTargetingInitiated))
    (Variables|Default|SetbTargetingInitiated true)
    (Utilities|Time|SetTimerbyEvent (delegate Custom|SelectTarget) (Math|Random|RandomFloatinRange (Variables|Default|GetTargetChangeDelayMin) (Variables|Default|GetTargetChangeDelayMax)) true)))

(event Custom|SelectTarget
  ;[1 1 1] Switching targets
  (Development|PrintString "Hello")
  (CallFunction|AssignTarget (CallFunction|GetRandomTarget)))

(event EventPossess
  (params (PossessedPawn :type Pawn%20Object%20Reference))
  (AI|RunBehaviorTree (Variables|Default|GetBTAsset))
  (bind _asenemy_base_bp (Utilities|Casting|CastToEnemyBase_BP PossessedPawn))
  (bind _output_get (Variables|Default|SetEnemyBase _asenemy_base_bp))
  (Utilities|IsValid (Variables|/Game/Blueprints/Pawns/Enemies/EnemyBase_BP.EnemyBase_BP_C|GetStartWaypoint _output_get)
    (:Is%20Valid
      (CallFunction|SetStartWaypoint (Variables|/Game/Blueprints/Pawns/Enemies/EnemyBase_BP.EnemyBase_BP_C|GetStartWaypoint _output_get)))))

(fn ConstructionScript)

(fn SetStartWaypoint
  (params (Waypoint :type Waypoint%20BP%20Object%20Reference))
  (AI|Components|Blackboard|SetValueasObject (Variables|Default|GetBlackboard) (Variables|Default|GetCurrentWaypointKey) Waypoint))

(fn AssignTarget
  (params (ObjectValue :type Object%20Object%20Reference))
  (bind _asactor (Utilities|Casting|CastToActor ObjectValue))
  (bind _targets (Variables|Default|GetTargets))
  (AI|Components|Blackboard|SetValueasObject (Variables|Default|GetBlackboard) (Variables|Default|GetCurrentTargetKey) ObjectValue)
  (Variables|Default|SetCurrentTarget _asactor)
  (CallFunction|InitiateTargeting)
  (if (not (Utilities|Array|ContainsItem _targets 0))
    (Utilities|Array|AddUnique _targets _asactor)))

(fn AddNewTarget
  (params (Target :type Actor%20Object%20Reference%20%28by%20ref%29))
  (Utilities|Array|AddUnique (Variables|Default|GetTargets) Target))

(fn GetRandomTarget
  (bind _targets (Variables|Default|GetTargets))
  (return (Utilities|Array|Get(acopy) _targets (Math|Random|RandomIntegerinRange 0 (- (Utilities|Array|Length _targets) 1)))))