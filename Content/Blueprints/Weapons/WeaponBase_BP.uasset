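; Base weapon Blueprint that fires projectile actors automatically while the trigger is held.
; StartFire fires one shot immediately and opens a Tick gate that fires again at the FireRate interval until StopFire closes it.
; Each shot plays an optional montage and spawns a projectile, passing it damage, instigator and weapon reference.
; Projectiles leave BulletSpawnLocation, aimed by either that component's rotation or the owning pawn's control rotation.
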(event EventTick
  (params (DeltaSeconds :type Float%20%28single-precision%29))
  (|CallParentFunction DeltaSeconds)
  (Utilities|FlowControl|Gate true
    (:Exit
      (bind _output_get (Variables|Default|SetFireTimer (+ (Variables|Default|GetFireTimer) (Utilities|Time|GetWorldDeltaSeconds))))
      (if (> _output_get (/ 1.0 (Variables|Default|GetFireRate)))
        (CallFunction|FireSingleShot)))))

(event EventStartFire
  (if (not (Variables|Default|GetbIsFiring))
    (Variables|Default|SetbIsFiring true)
    (CallFunction|FireSingleShot)
    (Utilities|FlowControl|Gate true) ; enters at Open
  ))

(event EventStopFire
  (Variables|Default|SetbIsFiring false)
  (Utilities|FlowControl|Gate true) ; enters at Close
)

(fn ConstructionScript)

(fn TryPlayFireMontage
  (bind _weaponfiremontage (Variables|Default|GetWeaponFireMontage))
  (bind _animatedmesh (Variables|Default|GetAnimatedMesh))
  (Utilities|IsValid _animatedmesh
    (:Is%20Valid
      (Utilities|IsValid _weaponfiremontage
        (:Is%20Valid
          (Animation|Montage|MontagePlay (Components|SkeletalMesh|GetAnimInstance _animatedmesh) _weaponfiremontage 1.0 "MontageLength" 0.0 true))
        (:Is%20Not%20Valid
          _)))
    (:Is%20Not%20Valid
      _))
  (return))

(fn GetProjectileTransform
  (bind _bulletspawnlocation (Variables|Default|GetBulletSpawnLocation))
  (if (Variables|Default|GetbAimAtControlRotation)
    (return (Math|Transform|MakeTransform (Transformation|GetWorldLocation _bulletspawnlocation) (Pawn|GetControlRotation (Variables|Default|GetWeaponPawnOwner) :!class /Script/Engine.Pawn)))
    (else
      (return (Math|Transform|MakeTransform (Transformation|GetWorldLocation _bulletspawnlocation) (Transformation|GetWorldRotation _bulletspawnlocation))))))

(fn FireSingleShot
  (Variables|Default|SetFireTimer 0.0)
  (CallFunction|TryPlayFireMontage)
  (Game|SpawnActorfromClass (Variables|Default|GetProjectile) (CallFunction|GetProjectileTransform) "Undefined" 0 self (Variables|Default|GetDamageInstigator) (Variables|Default|GetDamage) 0))