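; Base weapon projectile that plays a shot sound on spawn and damages what it hits.
; On BeginPlay it queries the weapon owner's team through GetTeamTypeMessage and sets collision object type and responses, so each team's projectiles ignore their own channel and block the opposing one.
; The first hit on anything but the owner applies point damage, pushes physics-simulating components along its velocity, spawns a hit particle and destroys the projectile.
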(event EventBeginPlay
  (Audio|PlaySoundatLocation (Variables|Default|GetShotSound) (Transformation|GetActorLocation) "0, 0, 0" 1.0 1.0 0.0 0 0 0)
  (CallFunction|SetupCollision))

(event Collision|EventHit
  (params (MyComp :type Primitive%20Component%20Object%20Reference) (Other :type Actor%20Object%20Reference) (OtherComp :type Primitive%20Component%20Object%20Reference) (bSelfMoved :type Boolean) (HitLocation :type Vector :default "0, 0, 0") (HitNormal :type Vector :default "0, 0, 0") (NormalImpulse :type Vector :default "0, 0, 0") (Hit :type Hit%20Result%20Structure%20%28by%20ref%29))
  (bind _weaponreference (Variables|Default|GetWeaponReference))
  (Utilities|IsValid _weaponreference
    (:Is%20Valid
      (if (!= Other (Variables|/Game/Blueprints/Weapons/WeaponBase_BP.WeaponBase_BP_C|GetWeaponOwner _weaponreference))
        (if (not (Variables|Default|GetbHit))
          (Variables|Default|SetbHit true)
          (Utilities|FlowControl|Sequence
            (:then_0
              ;[1 1 1] Damage
              (Game|Damage|ApplyPointDamage Other (Variables|Default|GetDamage) (Variables|/Script/Engine.MovementComponent|GetVelocity (Variables|Default|GetProjectileMovement)) Hit (Variables|Default|GetDamageInstigator) self))
            (:then_1
              ;[1 1 1] Physical Impulse
              (Utilities|IsValid OtherComp
                (:Is%20Valid
                  (if (Physics|IsSimulatingPhysics OtherComp "None")
                    (Physics|AddImpulseatLocation OtherComp (* (Transformation|GetVelocity) 1e+02) (Transformation|GetActorLocation) "None")))))
            (:then_2
              ;[0 1 0.1293] FX
              (Effects|SpawnEmitteratLocation (Variables|Default|GetHitParticle) HitLocation "0, 0, 0" "2.000000,2.000000,2.000000"))
            (:then_3
              (Actor|DestroyActor))))))))

(fn ConstructionScript)

(fn SetupCollision
  (bind _collision (Variables|Default|GetCollision))
  (bind _collision_2 (Variables|Default|GetCollision))
  (bind _weaponreference (Variables|Default|GetWeaponReference))
  (bind _weaponowner (Variables|/Game/Blueprints/Weapons/WeaponBase_BP.WeaponBase_BP_C|GetWeaponOwner _weaponreference))
  (Utilities|IsValid _weaponreference
    (:Is%20Valid
      (Utilities|IsValid _weaponowner
        (:Is%20Valid
          (bind _teamtype (Class|TeamInterfaceBP|GetTeamType(Message) _weaponowner))
          (switch Utilities|FlowControl|Switch|SwitchonE_TeamType _teamtype
            (:NewEnumerator0
              (Collision|SetCollisionObjectType _collision_2 "ECC_GameTraceChannel2")
              (Collision|SetCollisionResponsetoChannel _collision_2 "ECC_Pawn" "ECR_Block")
              (Collision|SetCollisionResponsetoChannel _collision_2 "ECC_GameTraceChannel3" "ECR_Block")
              (Collision|SetCollisionResponsetoChannel _collision_2 "ECC_GameTraceChannel2" "ECR_Ignore"))
            (:NewEnumerator1
              (Collision|SetCollisionObjectType _collision "ECC_GameTraceChannel3")
              (Collision|SetCollisionResponsetoChannel _collision "ECC_Pawn" "ECR_Ignore")
              (Collision|SetCollisionResponsetoChannel _collision "ECC_GameTraceChannel3" "ECR_Ignore")
              (Collision|SetCollisionResponsetoChannel _collision "ECC_GameTraceChannel2" "ECR_Block"))))))))