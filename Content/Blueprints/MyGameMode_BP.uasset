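; Game mode Blueprint that sets up the player HUD and ends the game when the Blueprint rush quest completes or fails.
; On start it creates the HUD widget, hands it to the player character, clears sound mixes and resets quests.
; It listens for quest state changes; either outcome disables player input, damage and weapon ticking, then fades screen and audio before reloading Level_01_ALL by name.
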(event Custom|OnQuestStateChanged_Event
  (params (Quest :type Quest%20Object%20Reference) (NewState :type EQuestState%20Enum :default "INACTIVE") (bIsCurrentQuest :type Boolean))
  (bind _returnvalue (Class|GlobalFunctionLibrary|GetMyPlayerCharacter))
  (if (== (Variables|/Script/QuestSystem.Quest|GetQuestSubclass Quest) "/Game/Blueprints/Objectives/BlueprintRushQuest_BP.BlueprintRushQuest_BP_C")
    (switch Utilities|FlowControl|Switch|SwitchonEQuestState NewState
      (:COMPLETED
        _)
      (:FAILED
        _))
    (Default|CallOnGameEnd)
    (Input|DisableInput _returnvalue (Game|GetPlayerController 0))
    (Variables|/Script/Game_02.HealthComponent|SetbCanBeDamaged (Variables|/Script/Game_02.MyPlayerCharacter|GetHealthComponent _returnvalue) false)
    (Actor|Tick|SetActorTickEnabled (Variables|/Script/Game_02.WeaponComponent|GetWeaponRef (Variables|/Script/Game_02.MyPlayerCharacter|GetWeaponComponent _returnvalue)))
    (Utilities|FlowControl|Delay 2.0)
    (Class|QuestSubsystem|DeactivateQuestMarker (Subsystems|GetQuestSubsystem) "/Game/Blueprints/Objectives/BlueprintRushQuest_BP.BlueprintRushQuest_BP_C")
    (CameraFades|StartCameraFade :self (Game|GetPlayerCameraManager 0) :ToAlpha 1.0 :Duration 2.0 :bHoldWhenFinished true)
    (Audio|PushSoundMixModifier "/Game/Audio/Sounds/Mixes/FadeOutSFX_SoundMix.FadeOutSFX_SoundMix")
    (Utilities|FlowControl|Delay 4.0)
    (Game|OpenLevel(byName) "Level_01_ALL")))

(event EventBeginPlay
  (bind _returnvalue (Subsystems|GetQuestSubsystem))
  (|CallParentFunction)
  (Class|GameplayStatics|ClearSoundMixModifiers)
  (EventDispatchers|AssignOnQuestStateChanged _returnvalue (delegate Custom|OnQuestStateChanged_Event))
  (Class|QuestSubsystem|ClearQuests _returnvalue))

(event EventOnStartPlay
  (CallFunction|CreateHUD))

(fn ConstructionScript)

(fn CreateHUD
  (bind _returnvalue (UserInterface|CreateWidget "/Game/UI/HUD/WB_PlayerHUD.WB_PlayerHUD_C" (Game|GetPlayerController 0)))
  (bind _output_get (Variables|Default|SetPlayerHUD _returnvalue))
  (UserInterface|Viewport|AddtoPlayerScreen _output_get)
  (bind _asmy_player_character_bp (Utilities|Casting|CastToMyPlayerCharacter_BP (Game|Player|GetPlayerPawn 0)))
  (bind _output_get_2 (Variables|Default|SetPlayerCharacterBP _asmy_player_character_bp))
  (Default|InitHUD _output_get_2 (Variables|Default|GetPlayerHUD)))