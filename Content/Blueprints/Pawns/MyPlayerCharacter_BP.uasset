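; Player character pawn Blueprint that sets up weapon, aiming cursor and input-device handling, and handles player death.
; BeginPlay initializes the weapon component and shows either the gamepad aim widget or the world cursor, while key presses notify the GameInstance and toggle the mouse cursor by device.
; On death it stops and hides the weapon, disables input, then fails the rush quest after a short delay.
; It also feeds Health to the HUD, reports its team and quits on Escape.
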(event Custom|OnDeathEvent
  (bind _weaponcomponent_bp (Variables|Default|GetWeaponComponent_BP))
  ;[1 1 1] Player death
  (Default|CallOnPlayerDeath)
  (Actor|Tick|SetActorTickEnabled false)
  (Actor|Tick|SetActorTickEnabled (Variables|/Script/Game_02.WeaponComponent|GetWeaponRef _weaponcomponent_bp))
  (Class|WeaponComponent|StopFire _weaponcomponent_bp)
  (Input|DisableInput (Game|GetPlayerController 0))
  (Rendering|SetActorHiddenInGame (Variables|/Script/Game_02.WeaponComponent|GetWeaponRef (Variables|Default|GetWeaponComponent_BP)) true)
  (Collision|SetCollisionResponsetoChannel (Variables|Default|GetCapsuleComponent) "ECC_GameTraceChannel3" "ECR_Ignore")
  (Utilities|FlowControl|Delay 1.0)
  (Class|QuestSubsystem|FinishQuest (Subsystems|GetQuestSubsystem) "/Game/Blueprints/Objectives/BlueprintRushQuest_BP.BlueprintRushQuest_BP_C" "FAILED"))

(event EventBeginPlay
  (bind _returnvalue (Game|GetPlayerController 0))
  (bind _gamepadaimwidget (Variables|Default|GetGamepadAimWidget))
  (bind _cursortoworld (Variables|Default|GetCursorToWorld))
  (bind _mesh (Variables|Character|GetMesh))
  ;[1 1 1] Initial settings
  (|CallParentFunction)
  (Class|WeaponComponent|InitWeapon (Variables|Default|GetWeaponComponent_BP) _mesh (Game|GetPlayerController 0) self _mesh)
  (EventDispatchers|AssignOnDeath (Variables|Default|GetHealth) (EventDispatchers|CreateEvent :!event Custom|OnDeathEvent))
  (if (Class|GlobalFunctionLibrary|IsGamepadUsed)
    (Variables|/Script/Engine.PlayerController|SetbShowMouseCursor _returnvalue false)
    (Rendering|SetVisibility _gamepadaimwidget true false)
    (Rendering|SetVisibility _cursortoworld false false)
    (else
      (Variables|/Script/Engine.PlayerController|SetbShowMouseCursor _returnvalue true)
      (Rendering|SetVisibility _gamepadaimwidget false false)
      (Rendering|SetVisibility _cursortoworld true false))))

(event EventPossessed
  (params (NewController :type Controller%20Object%20Reference))
  ;[1 1 1] Initial settings
  (Actor|Tick|AddTickPrerequisiteActor NewController))

(event Input|KeyboardEvents|Escape
  (params (Key :type Key%20Structure :default "None"))
  ;[0 0.9386 1] Quit game
  (:Pressed
    (Game|QuitGame 0 "Quit" false)))

(event Input|KeyboardEvents|AnyKey
  (params (Key :type Key%20Structure :default "None"))
  (bind _returnvalue (Class|GlobalFunctionLibrary|GetMyGameInstance))
  (bind _returnvalue_2 (Class|KismetInputLibrary|KeyIsGamepadKey Key))
  ;[0 1 0.9826] Detecting input
  (:Pressed
    (if (not (Class|KismetInputLibrary|KeyIsAnalog Key))
      (Default|CallOnAnyKeyPressed _returnvalue)
      (Class|MyGameInstance|OnAnyKey _returnvalue _returnvalue_2)
      (Variables|/Script/Engine.PlayerController|SetbShowMouseCursor (Game|GetPlayerController 0) (not _returnvalue_2)))))

(event Input|GamepadEvents|GamepadSpecialRight
  (params (Key :type Key%20Structure :default "None"))
  ;[0 0.9386 1] Quit game
  (:Pressed
    (Game|QuitGame 0 "Quit" false)))

(fn ConstructionScript)

(fn InitHUD
  (params (PlayerHUD :type WB%20Player%20HUD%20Object%20Reference))
  (Default|Initialize (Variables|/Game/UI/HUD/WB_PlayerHUD.WB_PlayerHUD_C|GetWB_PlayerHealth PlayerHUD) (Variables|Default|GetHealth))
  (Variables|Default|SetPlayerHUD PlayerHUD))

(fn GetTeamType
  (return (Variables|Default|GetTeamType)))