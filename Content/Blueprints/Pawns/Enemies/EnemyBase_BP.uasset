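; EnemyBase_BP is the base enemy pawn, with a health component, weapon component, floating movement and team type.
; On possession it caches its AI controller, which receives targets from damage instigators or forced calls.
; Damage from a valid instigator shows a 3D health bar that hides after a retriggerable delay.
; Death notifies the controller, halts fire and movement, plays explosion effects, broadcasts OnDeath, then destroys the actor.
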(event Custom|OnDeath_Event_0
  (bind _returnvalue (Transformation|GetActorLocation))
  ;[1 1 1] Death
  (Default|OnPawnDeath (Variables|Default|GetAIControllerBase))
  (CallFunction|StopFire)
  (Class|NavMovementComponent|StopActiveMovement (Variables|Default|GetFloatingPawnMovement))
  (Effects|SpawnEmitteratLocation "/Game/Effects/StarterContent/Particles/P_Explosion.P_Explosion" _returnvalue "0, 0, 0" "2.000000,2.000000,2.000000")
  (Audio|PlaySoundatLocation "/Game/Audio/Sounds/Explosions/Explosion_Cue.Explosion_Cue" _returnvalue "0, 0, 0" 1.5 1.0 0.0 0 0 0)
  (Default|CallOnDeath)
  (Utilities|FlowControl|Delay 0.2)
  (Actor|DestroyActor))

(event Custom|StopFire
  ;[1 1 1] Shooting
  (Class|WeaponComponent|StopFire (Variables|Default|GetWeaponComponent_BP)))

(event Custom|ForceTarget
  (params (Target :type Object%20Object%20Reference))
  ;[1 1 1] Forcing target
  (Default|AssignTarget (Variables|Default|GetAIControllerBase) Target))

(event Custom|Fire
  ;[1 1 1] Shooting
  (Class|WeaponComponent|StartFire (Variables|Default|GetWeaponComponent_BP)))

(event Game|Damage|EventAnyDamage
  (params (Damage :type Float%20%28single-precision%29) (DamageType :type Damage%20Type%20Object%20Reference) (InstigatedBy :type Controller%20Object%20Reference) (DamageCauser :type Actor%20Object%20Reference))
  ;[1 1 1] Targeting damage instigator
  (Utilities|IsValid InstigatedBy
    (:Is%20Valid
      (Default|AssignTarget (Variables|Default|GetAIControllerBase) (Pawn|GetControlledPawn InstigatedBy))
      (Widget|SetVisibility (Variables|Default|GetHealthBarRef) "Visible")
      (Utilities|FlowControl|RetriggerableDelay 3.0)
      (Widget|SetVisibility (Variables|Default|GetHealthBarRef) "Hidden"))))

(event EventPossessed
  (params (NewController :type Controller%20Object%20Reference))
  ;[1 1 1] Initial settings
  (bind _asaicontroller_base_bp (Utilities|Casting|CastToAIControllerBase_BP NewController))
  (Variables|Default|SetAIControllerBase _asaicontroller_base_bp))

(event EventBeginPlay
  ;[1 1 1] Initial settings
  (EventDispatchers|AssignOnDeath (Variables|Default|GetHealth) (EventDispatchers|CreateEvent :!event Custom|OnDeath_Event_0))
  (bind _aswb_health_bar_3d (Utilities|Casting|CastToWB_HealthBar3D (UserInterface|GetUserWidgetObject (Variables|Default|GetHealthBar))))
  (bind _output_get (Variables|Default|SetHealthBarRef _aswb_health_bar_3d))
  (Default|Initialize _output_get (Variables|Default|GetHealth))
  (Widget|SetVisibility _output_get "Collapsed"))

(fn ConstructionScript)

(fn GetTeamType
  (return (Variables|Default|GetTeamType)))