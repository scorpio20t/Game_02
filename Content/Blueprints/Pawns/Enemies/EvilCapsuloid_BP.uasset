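; EvilCapsuloid is an enemy pawn with two guns, a spotlight and glowing eyes.
; On BeginPlay it initializes left and right weapon components at their attach points, with the AI controller as damage instigator, and creates dynamic eye materials.
; Fire alternates between the two guns through a FlipFlop, while StopFire stops both.
; ChangeSpotlightColor tints the spotlight and both eyes together.
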(event Custom|ChangeSpotlightColor
  (params (NewLightColor :type Linear%20Color%20Structure))
  (Rendering|Components|Light|SetLightColor (Variables|Default|GetSpotLight) NewLightColor true)
  (Rendering|Material|SetVectorParameterValue (Variables|Default|GetEyeRMat) "Color" NewLightColor :!class /Script/Engine.MaterialInstanceDynamic))

(event EventBeginPlay
  (|CallParentFunction)
  (Class|WeaponComponent|InitWeapon (Variables|Default|GetWeaponComponent_BP) 0 (Variables|Default|GetAIControllerBase) self (Variables|Default|GetGunL_AttachPoint))
  (Class|WeaponComponent|InitWeapon (Variables|Default|GetWeaponComponent_BP_R) 0 (Variables|Default|GetAIControllerBase) self (Variables|Default|GetGunR_AttachPoint))
  (bind _returnvalue (Rendering|Material|CreateDynamicMaterialInstance (Variables|Default|GetEyeR) 0 "/Game/Materials/M_CubeoidEye.M_CubeoidEye" "None" :!class /Script/Engine.PrimitiveComponent))
  (Variables|Default|SetEyeRMat _returnvalue)
  (bind _returnvalue_2 (Rendering|Material|CreateDynamicMaterialInstance (Variables|Default|GetEyeL) 0 "/Game/Materials/M_CubeoidEye.M_CubeoidEye" "None" :!class /Script/Engine.PrimitiveComponent))
  (Variables|Default|SetEyeLMat _returnvalue_2))

(event EventFire
  (Utilities|FlowControl|FlipFlop
    (:A
      (Class|WeaponComponent|StartFire (Variables|Default|GetWeaponComponent_BP)))
    (:B
      (Class|WeaponComponent|StartFire (Variables|Default|GetWeaponComponent_BP_R)))))

(event EventStopFire
  (Class|WeaponComponent|StopFire (Variables|Default|GetWeaponComponent_BP)))

(fn ConstructionScript
  (|CallParentFunction))