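; Enemy pawn Blueprint for the Evil Capsuleoid, with two gun components, two eyes and a spotlight.
; BeginPlay initialises the left and right weapons on their attach points, with the AI controller as damage instigator, and creates dynamic eye materials.
; ChangeSpotlightColor applies the given color to the spotlight but always turns the eyes red.
; Looping test-fire timers for each gun remain in the graph, disconnected.
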(event Custom|CustomEvent_1
  ;[1 0.06014 0] TEST shooting
  (Default|Fire (Variables|Default|GetWeaponComponent_BP_R)))

(event Custom|CustomEvent_0
  ;[1 0.06014 0] TEST shooting
  (Default|Fire (Variables|Default|GetWeaponComponent_BP)))

(event Custom|ChangeSpotlightColor
  (params (NewLightColor :type Linear%20Color%20Structure))
  (Rendering|Components|Light|SetLightColor (Variables|Default|GetSpotLight) NewLightColor true)
  (Rendering|Material|SetVectorParameterValue (Variables|Default|GetEyeRMat) "Color" "(R=1.000000,G=0.000000,B=0.000000,A=1.000000)" :!class /Script/Engine.MaterialInstanceDynamic))

(event EventBeginPlay
  (|CallParentFunction)
  (Default|InitWeapon (Variables|Default|GetWeaponComponent_BP) 0 (Variables|Default|GetAIControllerBase) self (Variables|Default|GetGunL_AttachPoint))
  (Default|InitWeapon (Variables|Default|GetWeaponComponent_BP_R) 0 (Variables|Default|GetAIControllerBase) self (Variables|Default|GetGunR_AttachPoint))
  (bind _returnvalue (Rendering|Material|CreateDynamicMaterialInstance (Variables|Default|GetEyeR) 0 "/Game/Materials/M_CubeoidEye.M_CubeoidEye" "None" :!class /Script/Engine.PrimitiveComponent))
  (Variables|Default|SetEyeRMat _returnvalue)
  (bind _returnvalue_2 (Rendering|Material|CreateDynamicMaterialInstance (Variables|Default|GetEyeL) 0 "/Game/Materials/M_CubeoidEye.M_CubeoidEye" "None" :!class /Script/Engine.PrimitiveComponent))
  (Variables|Default|SetEyeLMat _returnvalue_2))

(fn ConstructionScript
  (|CallParentFunction))