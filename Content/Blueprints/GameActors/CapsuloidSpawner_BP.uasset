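; Spawner actor that releases waves of EvilCapsuloid_BP enemies at its own transform.
; SpawnEnemies loops with a delay until the target count is reached, then resets the counter so another wave can run.
; Each capsuloid receives the spawner's waypoint data, is forced to target the player pawn and is tracked in an array.
; DestroySpawnedCapsuloids applies heavy damage to every tracked capsuloid, crediting the player controller as instigator.
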(event Custom|SpawnEnemies
  (if (< (Variables|Default|GetSpawnedEnemies) (Variables|Default|GetEnemiesToSpawn)) :!label _label
    (bind _returnvalue (Game|SpawnActorfromClass "/Game/Blueprints/Pawns/Enemies/EvilCapsuloid_BP.EvilCapsuloid_BP_C" (Transformation|GetActorTransform) "Undefined" 0 (Variables|Default|GetBackgroundWaypoints) (Variables|Default|GetStartWaypoint) 0))
    (Utilities|Array|AddUnique (Variables|Default|GetSpawnedCapsuloids) _returnvalue)
    (Default|ForceTarget _returnvalue (Game|Player|GetPlayerPawn 0))
    (Math|Integer|IncrementInt (Variables|Default|GetSpawnedEnemies)
      (:%20%20
        (Utilities|FlowControl|Delay (Variables|Default|GetDelayBetweenSpawns))
        (goto _label)))
    (else
      ;[1 1 1] So we can spawn again
      (Variables|Default|SetSpawnedEnemies 0))))

(event Custom|DestroySpawnedCapsuloids
  (for _array_element (Variables|Default|GetSpawnedCapsuloids)
    (Game|Damage|ApplyDamage _array_element 5e+03 (Game|GetPlayerController 0) (Components|GetOwner))))

(fn ConstructionScript)