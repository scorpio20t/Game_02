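; FlawlessBlueprint_BP is a game actor with a Health component and a 3D health bar widget that explodes when it dies.
; On BeginPlay it initializes the WB_HealthBar3D widget with Health and binds to that component's death event, both only if the widget cast succeeds.
; On death it spawns an enlarged explosion effect and sound, broadcasts OnDeath, then destroys itself after a short delay.
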(event Custom|OnDeath_Event_0
  (bind _returnvalue (Transformation|GetActorLocation))
  (Effects|SpawnEmitteratLocation "/Game/StarterContent/Particles/P_Explosion.P_Explosion" _returnvalue "0, 0, 0" "3.000000,3.000000,3.000000")
  (Audio|PlaySoundatLocation "/Game/Audio/Sounds/Explosions/Explosion_Cue.Explosion_Cue" _returnvalue "0, 0, 0" 2.0 0.8 0.0 0 0 0)
  (Default|CallOnDeath)
  (Utilities|FlowControl|Delay 0.2)
  (Actor|DestroyActor))

(event EventBeginPlay
  (bind _health (Variables|Default|GetHealth))
  (bind _aswb_health_bar_3d (Utilities|Casting|CastToWB_HealthBar3D (UserInterface|GetUserWidgetObject (Variables|Default|GetHealthBar))))
  (Default|Initialize _aswb_health_bar_3d _health)
  (EventDispatchers|AssignOnDeath _health (delegate Custom|OnDeath_Event_0)))

(fn ConstructionScript)