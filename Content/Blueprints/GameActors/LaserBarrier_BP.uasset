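; LaserBarrier_BP is a laser gate actor that blocks passage with seven beam components and a spotlight.
; BeginPlay gathers the beams into an array.
; The Open event hides every beam, disables its collision and turns off the light.
; The Close event reverses this, showing the beams, restoring query and physics collision and relighting the spotlight.
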(event Custom|Open
  (for _array_element (Variables|Default|GetBeams)
    (Development|SetHiddeninGame _array_element true false)
    (Collision|SetCollisionEnabled _array_element "NoCollision"))
  (Rendering|SetVisibility (Variables|Default|GetSpotLight) false false))

(event Custom|Close
  (for _array_element (Variables|Default|GetBeams)
    (Development|SetHiddeninGame _array_element false false)
    (Collision|SetCollisionEnabled _array_element "QueryAndPhysics"))
  (Rendering|SetVisibility (Variables|Default|GetSpotLight) true false))

(event EventBeginPlay
  (Variables|Default|SetBeams (Utilities|Array|MakeArray (Variables|Default|GetBeam1) (Variables|Default|GetBeam2) (Variables|Default|GetBeam3) (Variables|Default|GetBeam4) (Variables|Default|GetBeam5) (Variables|Default|GetBeam6) (Variables|Default|GetBeam7))))

(fn ConstructionScript)