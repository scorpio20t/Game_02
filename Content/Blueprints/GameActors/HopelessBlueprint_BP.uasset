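; A rotating turret enemy with health, a 3D health bar, staged damage effects and an explosive death.
; Once activated on start or by a call, its left and right weapons fire independent random bursts while it lives, and its base spins faster as health drops.
; A player detection sphere triggers an animated, audible shockwave warm-up, then launches and damages the player if still inside, repeating while they stay.
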(event OnComponentBeginOverlap(PlayerDetectionSphere)
  (params (OverlappedComponent :type Primitive%20Component%20Object%20Reference) (OtherActor :type Actor%20Object%20Reference) (OtherComp :type Primitive%20Component%20Object%20Reference) (OtherBodyIndex :type Integer) (bFromSweep :type Boolean) (SweepResult :type Hit%20Result%20Structure%20%28by%20ref%29))
  ;[0.9792 0.9583 1] Shockwave
  (CallFunction|TryStartShockwaveSequence))

(event Custom|OnFinished_Event_0
  (bind _returnvalue (Game|GetPlayerCharacter 0))
  ;[0.9792 0.9583 1] Shockwave
  (Components|Activation|Deactivate (Variables|Default|GetAudio_WarmUp))
  (Audio|PlaySoundatLocation "/Game/Audio/Sounds/Objects/S_Shockwave_Cue.S_Shockwave_Cue" (Transformation|GetActorLocation) "0, 0, 0" 1.0 1.0 0.0 0 0 0)
  (Components|Activation|Activate (Variables|Default|GetP_AreaAttack_Shockwave) false)
  (if (Collision|IsOverlappingActor (Variables|Default|GetPlayerDetectionSphere) _returnvalue :!class /Script/Engine.PrimitiveComponent)
    (Character|LaunchCharacter _returnvalue (* (Math|Vector|GetUnitDirection(Vector) (Transformation|GetWorldLocation (Variables|Default|GetArrow2)) (Transformation|GetActorLocation _returnvalue)) 9e+02) false false)
    (Game|Damage|ApplyDamage _returnvalue 15.0 0 self)
    (Variables|Default|SetShockwaveSequenceInProgress false)
    (Utilities|FlowControl|Delay 3.0)
    (if (Collision|IsOverlappingActor (Variables|Default|GetPlayerDetectionSphere) (Game|GetPlayerCharacter 0) :!class /Script/Engine.PrimitiveComponent)
      (CallFunction|TryStartShockwaveSequence))
    (else
      (Variables|Default|SetShockwaveSequenceInProgress false))))

(event Custom|Activate
  ;[1 1 1] Random bursts
  (Actor|Tick|SetActorTickEnabled true)
  (Utilities|FlowControl|Sequence
    (:then_0
      (Class|WeaponComponent|StartFire (Variables|Default|GetWeaponComponent_BP_R) :!label _label)
      (Utilities|FlowControl|Delay (Math|Random|RandomFloatinRange 0.5 2.0))
      (Class|WeaponComponent|StopFire (Variables|Default|GetWeaponComponent_BP_R))
      (Utilities|FlowControl|Delay (Math|Random|RandomFloatinRange 1.0 2.0))
      (if (Variables|/Script/Game_02.HealthComponent|GetbIsAlive (Variables|Default|GetHealth))
        (goto _label)))
    (:then_1
      (Utilities|FlowControl|Delay 0.6)
      (Class|WeaponComponent|StartFire (Variables|Default|GetWeaponComponent_BP_L) :!label _label_2)
      (Utilities|FlowControl|Delay (Math|Random|RandomFloatinRange 0.5 2.0))
      (Class|WeaponComponent|StopFire (Variables|Default|GetWeaponComponent_BP_L))
      (Utilities|FlowControl|Delay (Math|Random|RandomFloatinRange 1.0 2.0))
      (if (Variables|/Script/Game_02.HealthComponent|GetbIsAlive (Variables|Default|GetHealth))
        (goto _label_2)))))

(event Custom|OnDeath_Event_0
  (bind _returnvalue (Transformation|GetActorLocation))
  (Class|WeaponComponent|StopFire (Variables|Default|GetWeaponComponent_BP_R))
  (Effects|SpawnEmitteratLocation "/Game/Effects/StarterContent/Particles/P_Explosion.P_Explosion" _returnvalue "0, 0, 0" "3.000000,3.000000,3.000000")
  (Audio|PlaySoundatLocation "/Game/Audio/Sounds/Explosions/Explosion_Cue.Explosion_Cue" _returnvalue "0, 0, 0" 2.0 0.8 0.0 0 0 0)
  (Default|CallOnDeath)
  (Utilities|FlowControl|Delay 0.2)
  (Actor|DestroyActor))

(event Custom|TryStartShockwaveSequence
  (bind _actorsequence (Variables|Default|GetActorSequence))
  (bind _audio_warmup (Variables|Default|GetAudio_WarmUp))
  (bind _sequenceplayer (Variables|/Script/ActorSequence.ActorSequenceComponent|GetSequencePlayer _actorsequence))
  ;[0.9792 0.9583 1] Shockwave
  (if (not (Variables|Default|GetShockwaveSequenceInProgress))
    (Variables|Default|SetShockwaveSequenceInProgress true)
    (Utilities|FlowControl|Sequence
      (:then_0
        (Sequencer|Player|Play _sequenceplayer :!class /Script/MovieScene.MovieSceneSequencePlayer)
        (EventDispatchers|AssignOnFinished _sequenceplayer (delegate Custom|OnFinished_Event_0)))
      (:then_1
        ;;[0.03079 1 0] WarmUp SFX
        (Components|Activation|Activate _audio_warmup false)
        (bind _pitch (Timeline|WarpUpSFX PlayFromStart)
          (:Update
            (Audio|Components|Audio|SetPitchMultiplier _audio_warmup _pitch)))))))

(event EventBeginPlay
  (Components|Movement|SetUpdatedComponent (Variables|Default|GetRotatingMovement) (Variables|Default|GetTurretBase))
  (bind _aswb_health_bar_3d (Utilities|Casting|CastToWB_HealthBar3D (UserInterface|GetUserWidgetObject (Variables|Default|GetHealthBar))))
  (Default|Initialize _aswb_health_bar_3d (Variables|Default|GetHealth))
  (Class|WeaponComponent|InitWeapon (Variables|Default|GetWeaponComponent_BP_R) 0 0 self (Variables|Default|GetAttachR))
  (Class|WeaponComponent|InitWeapon (Variables|Default|GetWeaponComponent_BP_L) 0 0 self (Variables|Default|GetAttachL))
  (EventDispatchers|AssignOnDeath (Variables|Default|GetHealth) (delegate Custom|OnDeath_Event_0))
  (Default|InitDamageFX (Variables|Default|GetDamageFXComponent_BP) (Utilities|Array|MakeArray (Variables|Default|GetParticleSystem_Sparks) (Variables|Default|GetParticleSystem_Smoke) (Variables|Default|GetParticleSystem_Fire)))
  (if (Variables|Default|GetbActivateOnStart)
    (CallFunction|Activate)))

(event EventTick
  (params (DeltaSeconds :type Float%20%28single-precision%29))
  ;[1 1 1] Less HP = faster turret rotation
  (Variables|/Script/Engine.RotatingMovementComponent|SetRotationRate (Variables|Default|GetRotatingMovement) (Math|Rotator|MakeRotator 0.0 0.0 (Math|Float|MapRangeClamped (Class|HealthComponent|GetHealthPercentage (Variables|Default|GetHealth)) 1.0 0.0 1e+02 3e+02))))

(fn ConstructionScript)

(fn GetTeamType
  (return (Variables|Default|GetTeamType)))