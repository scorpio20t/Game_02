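; Broken bridge actor that the player repairs through an in-world panel widget shown while in interaction range.
; The panel refreshes checkboxes on approach and receives forwarded gamepad D-pad and face button input, with input enabled only when a gamepad is used.
; TryActivate checks usability, then plays the repair sequence and sounds, turns buttons green and marks it fixed, or plays an access-denied sound.
; After a short delay, activation disables the blocking collision and signals completion.
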(event OnInteractioninRange(InteractionComponent)
  (params (InteractingActor :type Actor%20Object%20Reference))
  ;[1 1 1] Player proximity detection
  (if (not (Variables|Default|GetbFixed))
    (Default|RefreshCheckboxes (Variables|Default|GetBridgePanel))
    (Rendering|SetVisibility (Variables|Default|GetBridgePanelWidget) true false)
    (if (Class|GlobalFunctionLibrary|IsGamepadUsed)
      (Default|FocusGamepad (Variables|Default|GetBridgePanel))
      (Input|EnableInput (Game|GetPlayerController 0)))))

(event OnInteractionOutOfRange(InteractionComponent)
  (params (InteractingActor :type Actor%20Object%20Reference))
  ;[1 1 1] Player proximity detection
  (Rendering|SetVisibility (Variables|Default|GetBridgePanelWidget) false false)
  (Class|WidgetBlueprintLibrary|SetFocustoGameViewport)
  (Input|DisableInput (Game|GetPlayerController 0)))

(event Custom|ActivateBridge
  ;[1 1 1] Bridge interaction
  (Sequencer|Player|Play (Variables|/Script/ActorSequence.ActorSequenceComponent|GetSequencePlayer (Variables|Default|GetActorSequence)) :!class /Script/MovieScene.MovieSceneSequencePlayer)
  (Rendering|SetVisibility (Variables|Default|GetBridgePanelWidget) false false)
  (Rendering|Material|SetMaterial (Variables|Default|GetButton1) 0 "/Game/Materials/M_EmissiveGreen.M_EmissiveGreen")
  (Variables|Default|SetbFixed true)
  (Utilities|FlowControl|Delay 1.5)
  (Collision|SetCollisionEnabled (Variables|Default|GetCollision) "NoCollision")
  (Default|CallOnBridgeActivated))

(event Custom|TryActivate
  ;[1 1 1] Bridge interaction
  (if (Math|Boolean|ANDBoolean (not (Variables|Default|GetPlayerCannotUse)) (Variables|Default|GetIsNotInactive) (Variables|Default|GetNotInteractiveModeDisabled))
    (CallFunction|ActivateBridge)
    (Audio|PlaySoundatLocation "/Game/Audio/Sounds/Objects/S_Bridge_Cue.S_Bridge_Cue" (Transformation|GetActorLocation) "0, 0, 0" 1.0 1.0 0.0 0 0 0)
    (Audio|PlaySound2D "/Game/Audio/Sounds/Objects/S_NewObjective_Cue.S_NewObjective_Cue" 0.7 1.25 0.0 0 0)
    (else
      (Audio|PlaySound2D "/Game/Audio/Sounds/Objects/S_AccessDenied_1_Cue.S_AccessDenied_1_Cue" 1.0 1.0 0.0 0 0))))

(event EventBeginPlay
  (Class|InteractionComponent|SetInteractionCollision (Variables|Default|GetInteractionComponent) (Variables|Default|GetSphere))
  (bind _aswb_bridge_panel (Utilities|Casting|CastToWB_BridgePanel (UserInterface|GetUserWidgetObject (Variables|Default|GetBridgePanelWidget))))
  (bind _output_get (Variables|Default|SetBridgePanel _aswb_bridge_panel))
  (Default|Init _output_get self)
  (Rendering|SetVisibility (Variables|Default|GetBridgePanelWidget) false false))

(event Input|GamepadEvents|GamepadDPadDown
  (params (Key :type Key%20Structure :default "None"))
  ;[1 1 1] Widget Input
  (:Pressed
    (Default|DpadDown (Variables|Default|GetBridgePanel))))

(event Input|GamepadEvents|GamepadDPadUp
  (params (Key :type Key%20Structure :default "None"))
  ;[1 1 1] Widget Input
  (:Pressed
    (Default|DpadUp (Variables|Default|GetBridgePanel))))

(event Input|GamepadEvents|GamepadFaceButtonLeft
  (params (Key :type Key%20Structure :default "None"))
  ;[1 1 1] Widget Input
  (:Pressed
    (Default|GamepadFaceLeftPressed (Variables|Default|GetBridgePanel))))

(event Input|GamepadEvents|GamepadFaceButtonBottom
  (params (Key :type Key%20Structure :default "None"))
  ;[1 1 1] Widget Input
  (:Pressed
    (Default|GamepadFaceBottomPressed (Variables|Default|GetBridgePanel))))

(fn ConstructionScript)